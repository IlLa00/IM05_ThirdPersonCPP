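; BP_CAttachment_MagicBall is the equipment attachment that shows a magic ball particle effect on the character.
; On BeginPlay it attaches its particle system to the Hand_ThrowItem socket.
; Equipping activates the particles and plays a timeline that drives their relative scale, while unequipping deactivates them.
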(event EventBeginPlay
  (Class|CAttachment|ComponentAttachto (Variables|Default|GetParticleSystem) "Hand_ThrowItem"))

(event EventOnEquip
  (Components|Activation|SetActive (Variables|Default|GetParticleSystem) true false)
  (bind _output (Timeline|OnEquipTimeline PlayFromStart)
    (:Update
      (Transformation|SetRelativeScale3D (Variables|Default|GetParticleSystem) (Math|Conversions|ToVector(Float) _output)))))

(event EventOnUnequip
  (Components|Activation|SetActive (Variables|Default|GetParticleSystem) false false))

(fn ConstructionScript)