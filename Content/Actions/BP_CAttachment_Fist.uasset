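; BP_CAttachment_Fist is the fist attachment actor for the action system, providing sphere components and particle effects tied to equip state.
; On BeginPlay it attaches every sphere component to the socket that shares the component's object name, so component naming determines placement.
; OnEquip activates all of its particle system components without resetting them, and OnUnequip deactivates them.
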(event EventBeginPlay
  (for _array_element (Actor|GetComponentsByClass "/Script/Engine.SphereComponent")
    (Class|CAttachment|ComponentAttachto _array_element (Utilities|String|StringToName (Utilities|GetObjectName _array_element)))))

(event EventOnEquip
  (for _array_element (Actor|GetComponentsByClass "/Script/Engine.ParticleSystemComponent")
    (Components|Activation|SetActive _array_element true false)))

(event EventOnUnequip
  (for _array_element (Actor|GetComponentsByClass "/Script/Engine.ParticleSystemComponent")
    (Components|Activation|SetActive _array_element false false)))

(fn ConstructionScript)